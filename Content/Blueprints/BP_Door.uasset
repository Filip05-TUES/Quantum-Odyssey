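; BP_Door is a door that shows a text prompt when the player is holding a key at it while it is closed.
; BeginPlay caches the player as a BP_SpriteCharacter.
; Overlap events track IsOverlapped and toggle the TextRender, checking the held item's class against BP_Key and the flipbook against FB_DoorClosed, so the sprite doubles as door state.
; The graph contains no logic to open the door.
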(event Collision|EventActorBeginOverlap
  (params (OtherActor :type Actor%20Object%20Reference))
  (Variables|Default|SetIsOverlapped true)
  (if (Math|Boolean|ANDBoolean (Variables|/Game/Blueprints/BP_SpriteCharacter.BP_SpriteCharacter_C|GetIsHoldingSomething (Variables|Default|GetPlayer)) (== (Utilities|GetClass (Variables|/Game/Blueprints/BP_SpriteCharacter.BP_SpriteCharacter_C|GetItemHeld (Variables|Default|GetPlayer))) "/Game/Blueprints/BP_Key.BP_Key_C") (== (Class|PaperFlipbookComponent|GetFlipbook (Variables|Default|GetSprite)) "/Game/Assets/environment/props/Door/FB_DoorClosed.FB_DoorClosed"))
    (Rendering|SetVisibility (Variables|Default|GetTextRender) true false)))

(event Collision|EventActorEndOverlap
  (params (OtherActor :type Actor%20Object%20Reference))
  (Variables|Default|SetIsOverlapped false)
  (Rendering|SetVisibility (Variables|Default|GetTextRender) false false))

(event EventBeginPlay
  (bind _asbp_sprite_character (Utilities|Casting|CastToBP_SpriteCharacter (Game|GetPlayerCharacter 0)))
  (Variables|Default|SetPlayer _asbp_sprite_character))

(fn ConstructionScript)