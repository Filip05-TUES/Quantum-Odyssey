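; BP_Trapdoor is a sprite-based trapdoor that opens when something overlaps its Box component.
; Box begin and end overlap set IsOpen, and Tick polls it to swap between open and closed sprites.
; Updates pause while the player's BP_SpriteCharacter is using its first ability.
; Opening disables the sprite's collision, and closing does not re-enable it.
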(event OnComponentBeginOverlap(Box)
  (params (OverlappedComponent :type Primitive%20Component%20Object%20Reference) (OtherActor :type Actor%20Object%20Reference) (OtherComp :type Primitive%20Component%20Object%20Reference) (OtherBodyIndex :type Integer) (bFromSweep :type Boolean) (SweepResult :type Hit%20Result%20Structure%20%28by%20ref%29))
  (Variables|Default|SetIsOpen true))

(event OnComponentEndOverlap(Box)
  (params (OverlappedComponent :type Primitive%20Component%20Object%20Reference) (OtherActor :type Actor%20Object%20Reference) (OtherComp :type Primitive%20Component%20Object%20Reference) (OtherBodyIndex :type Integer))
  (Variables|Default|SetIsOpen false))

(event Custom|UpdateTrapdoor
  (bind _asbp_sprite_character (Utilities|Casting|CastToBP_SpriteCharacter (Game|GetPlayerCharacter 0)))
  (if (not (Utilities|Array|Get(acopy) (Variables|/Game/Blueprints/BP_SpriteCharacter.BP_SpriteCharacter_C|GetIsAbilityBeingUsed _asbp_sprite_character)))
    (if (Variables|Default|GetIsOpen)
      (Rendering|Components|Sprite|SetSprite (Variables|Default|GetRenderComponent) "/Game/Assets/environment/props/Trapdoor/trapdoor_opened_Sprite.trapdoor_opened_Sprite")
      (Collision|SetCollisionEnabled (Variables|Default|GetRenderComponent) "NoCollision")
      (else
        (Rendering|Components|Sprite|SetSprite (Variables|Default|GetRenderComponent) "/Game/Assets/environment/props/Trapdoor/trapdoor_closed_Sprite.trapdoor_closed_Sprite")))))

(event EventTick
  (params (DeltaSeconds :type Float%20%28single-precision%29))
  (CallFunction|UpdateTrapdoor))

(fn ConstructionScript)