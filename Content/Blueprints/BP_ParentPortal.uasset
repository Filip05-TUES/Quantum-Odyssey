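; Parent portal actor that moves the player to its destination level when they interact while overlapping it.
; Overlap toggles a text prompt and a flag that Tick polls to check the character's interact state.
; Portals showing the boss arena flipbook instead display a dialogue warning until every GameInstance ability (Quantum stones) is collected.
; Before opening the level, it saves abilities and first-time state to a save slot.
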(event Custom|TeleportPlayer
  (bind _returnvalue (Game|GetGameInstance))
  (bind _asbp_game_instance (Utilities|Casting|CastToBP_GameInstance _returnvalue))
  (bind _asbp_sprite_character (Utilities|Casting|CastToBP_SpriteCharacter (Game|GetPlayerCharacter 0)))
  (if (Variables|/Game/Blueprints/BP_SpriteCharacter.BP_SpriteCharacter_C|GetIsInteracting _asbp_sprite_character)
    (bind _returnvalue_2 (SaveGame|CreateSaveGameObject "/Game/Blueprints/BP_Save.BP_Save_C"))
    (Variables|/Game/Blueprints/BP_Save.BP_Save_C|SetHasAbilities _returnvalue_2 (Variables|/Game/Blueprints/BP_GameInstance.BP_GameInstance_C|GetHasAbilities _asbp_game_instance))
    (Variables|/Game/Blueprints/BP_Save.BP_Save_C|SetIsFirstTime _returnvalue_2 (Variables|/Game/Blueprints/BP_GameInstance.BP_GameInstance_C|GetIsFirstTime _asbp_game_instance))
    (SaveGame|SaveGametoSlot _returnvalue_2 "save")
    (Game|OpenLevel(byName) (Utilities|String|StringToName (Variables|Default|GetDestinationLevel)))))

(event Collision|EventActorBeginOverlap
  (params (OtherActor :type Actor%20Object%20Reference))
  (Variables|Default|SetIsOverlapped true)
  (Development|SetHiddeninGame (Variables|Default|GetTextRender) false false))

(event Collision|EventActorEndOverlap
  (params (OtherActor :type Actor%20Object%20Reference))
  (Variables|Default|SetIsOverlapped false)
  (Development|SetHiddeninGame (Variables|Default|GetTextRender) true false)
  (bind _notificationwidget (Variables|Default|GetNotificationWidget)
    (:then
      (Widget|RemovefromParent _notificationwidget))
    (:else)))

(event EventTick
  (params (DeltaSeconds :type Float%20%28single-precision%29))
  (if (Variables|Default|GetIsOverlapped)
    (if (== (Class|PaperFlipbookComponent|GetFlipbook (Variables|Default|GetSprite self)) "/Game/Assets/environment/props/Portals/FB_BossArenaPortal.FB_BossArenaPortal")
      (if (Utilities|Array|ContainsItem (Variables|/Game/Blueprints/BP_GameInstance.BP_GameInstance_C|GetHasAbilities (.AsBP%20Game%20Instance (Utilities|Casting|CastToBP_GameInstance (Game|GetGameInstance)))) false)
        (if (Utilities|IsValid (Variables|Default|GetNotificationWidget))
          _
          (else
            (bind _returnvalue (UserInterface|CreateWidget "/Game/Widgets/WB_Dialogue.WB_Dialogue_C"))
            (Rendering|Components|TextRender|SetText (Variables|/Game/Widgets/WB_Dialogue.WB_Dialogue_C|GetTalkText _returnvalue) "You have to collect all Quantum stones before facing the Quantum Devourer!")
            (Rendering|Components|TextRender|SetText (Variables|/Game/Widgets/WB_Dialogue.WB_Dialogue_C|GetTalkText_1 _returnvalue) "")))
        (UserInterface|Viewport|AddtoViewport _returnvalue 0)
        (Variables|Default|SetNotificationWidget _returnvalue)
        (else
          (CallFunction|TeleportPlayer :!label _label)))
      (else
        (goto _label)))))

(fn ConstructionScript)