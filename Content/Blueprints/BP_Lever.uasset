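; BP_Lever is a 2D Paper2D lever that shows a text prompt while an actor overlaps it.
; Every Tick polls the player's BP_SpriteCharacter, resetting the sprite and IsPulled whenever its first ability is not in use.
; While overlapped and the player is interacting, the lever swaps to its pulled flipbook, setting IsPulled only if that ability is active.
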(event Custom|PullLever
  (bind _asbp_sprite_character (Utilities|Casting|CastToBP_SpriteCharacter (Game|GetPlayerCharacter 0)))
  (if (Variables|/Game/Blueprints/BP_SpriteCharacter.BP_SpriteCharacter_C|GetIsInteracting _asbp_sprite_character)
    (Sprite|SetFlipbook (Variables|Default|GetSprite) "/Game/Assets/environment/props/Lever/FB_LeverPulled.FB_LeverPulled")
    (if (Utilities|Array|Get(acopy) (Variables|/Game/Blueprints/BP_SpriteCharacter.BP_SpriteCharacter_C|GetIsAbilityBeingUsed _asbp_sprite_character))
      (Variables|Default|SetIsPulled true))))

(event Custom|ResetLever
  (bind _asbp_sprite_character (Utilities|Casting|CastToBP_SpriteCharacter (Game|GetPlayerCharacter 0)))
  (if (not (Utilities|Array|Get(acopy) (Variables|/Game/Blueprints/BP_SpriteCharacter.BP_SpriteCharacter_C|GetIsAbilityBeingUsed _asbp_sprite_character)))
    (Sprite|SetFlipbook (Variables|Default|GetSprite) "/Game/Assets/environment/props/Lever/FB_LeverDefault.FB_LeverDefault")
    (Variables|Default|SetIsPulled false)))

(event Collision|EventActorBeginOverlap
  (params (OtherActor :type Actor%20Object%20Reference))
  (Variables|Default|SetIsOverlapped true)
  (Development|SetHiddeninGame (Variables|Default|GetTextRender) false false))

(event EventTick
  (params (DeltaSeconds :type Float%20%28single-precision%29))
  (CallFunction|ResetLever)
  (if (Variables|Default|GetIsOverlapped)
    (CallFunction|PullLever)))

(event Collision|EventActorEndOverlap
  (params (OtherActor :type Actor%20Object%20Reference))
  (Variables|Default|SetIsOverlapped false)
  (Development|SetHiddeninGame (Variables|Default|GetTextRender) true false))

(fn ConstructionScript)