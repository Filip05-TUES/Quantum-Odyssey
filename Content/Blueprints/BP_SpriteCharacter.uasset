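; Paper2D player character for a side-scrolling game with four realm-specific abilities: time manipulation, Quantum Forge, entanglement and echo.
; Tick picks the flipbook from movement and revive state and turns the controller by X velocity; input drives movement, pausing and held-action flags.
; Ability keys work only in their map, toggling an effect widget if unlocked and no other is active.
; Death flags revival on the GameInstance, clears abilities and saves.
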(event Custom|UpdatePlayerAnimation
  (bind _charactermovement (Variables|Character|GetCharacterMovement))
  (bind _velocity (Variables|/Script/Engine.MovementComponent|GetVelocity _charactermovement))
  (bind (_x _y _z) (Math|Vector|BreakVector _velocity))
  (bind _asbp_game_instance (Utilities|Casting|CastToBP_GameInstance (Game|GetGameInstance)))
  (Sprite|SetFlipbook (Variables|Default|GetSprite) (select (Variables|Default|GetIsUnableToMove) "/Game/Assets/sprites/player/idle/player-idle.player-idle" (select (> _z 0.0) "/Game/Assets/sprites/player/jump/player-jump.player-jump" (select (< _z 0.0) "/Game/Assets/sprites/player/jump/player-fall.player-fall" (select (!= _x 0.0) "/Game/Assets/sprites/player/run/player-run.player-run" (select (Variables|/Game/Blueprints/BP_GameInstance.BP_GameInstance_C|GetIsPlayerReviving _asbp_game_instance) "/Game/Assets/sprites/player/hurt/FB_PlayerRevive.FB_PlayerRevive" "/Game/Assets/sprites/player/idle/player-idle.player-idle")))))))

(event Custom|UpdatePlayerRotation
  (Utilities|IsValid (Pawn|GetController)
    (:Is%20Valid
      (Math|Float|CompareFloat (.X (Math|Vector|BreakVector (Variables|/Script/Engine.MovementComponent|GetVelocity (Variables|Character|GetCharacterMovement)))) 0.0
        (:>
          (Pawn|SetControlRotation (Pawn|GetController) (Math|Rotator|MakeRotator 0.0 0.0 0.0)))
        (:<
          (Pawn|SetControlRotation (Pawn|GetController) (Math|Rotator|MakeRotator 0.0 0.0 1.8e+02)))))))

(event Custom|CheckForDeath
  (bind _returnvalue (Game|GetGameInstance))
  (bind _asbp_game_instance (Utilities|Casting|CastToBP_GameInstance _returnvalue))
  (if (<= (Variables|Default|GetHealth) 0)
    (bind _asbp_game_instance_2 (Utilities|Casting|CastToBP_GameInstance (Game|GetGameInstance)))
    (Utilities|FlowControl|Delay 2.0)
    (Variables|/Game/Blueprints/BP_GameInstance.BP_GameInstance_C|SetIsPlayerDead _asbp_game_instance_2 true)
    (Variables|/Game/Blueprints/BP_GameInstance.BP_GameInstance_C|SetIsPlayerReviving _asbp_game_instance_2 true)
    (bind _asbp_game_instance_3 (Utilities|Casting|CastToBP_GameInstance (Game|GetGameInstance)))
    (Utilities|Array|SetArrayElem (Variables|/Game/Blueprints/BP_GameInstance.BP_GameInstance_C|GetHasAbilities _asbp_game_instance_3) 0 false)
    (Utilities|Array|SetArrayElem (Variables|/Game/Blueprints/BP_GameInstance.BP_GameInstance_C|GetHasAbilities _asbp_game_instance_3) 1 false)
    (Utilities|Array|SetArrayElem (Variables|/Game/Blueprints/BP_GameInstance.BP_GameInstance_C|GetHasAbilities _asbp_game_instance_3) 2 false)
    (Utilities|Array|SetArrayElem (Variables|/Game/Blueprints/BP_GameInstance.BP_GameInstance_C|GetHasAbilities _asbp_game_instance_3) 3 false)
    (bind _returnvalue_2 (SaveGame|CreateSaveGameObject "/Game/Blueprints/BP_Save.BP_Save_C"))
    (Variables|/Game/Blueprints/BP_Save.BP_Save_C|SetHasAbilities _returnvalue_2 (Variables|/Game/Blueprints/BP_GameInstance.BP_GameInstance_C|GetHasAbilities _asbp_game_instance))
    (Variables|/Game/Blueprints/BP_Save.BP_Save_C|SetIsFirstTime _returnvalue_2 (Variables|/Game/Blueprints/BP_GameInstance.BP_GameInstance_C|GetIsFirstTime _asbp_game_instance))
    (SaveGame|SaveGametoSlot _returnvalue_2 "save")))

(event EventTick
  (params (DeltaSeconds :type Float%20%28single-precision%29))
  (CallFunction|UpdatePlayerAnimation)
  (CallFunction|UpdatePlayerRotation))

(event Input|ActionEvents|InputActionJump
  (params (Key :type Key%20Structure :default "None"))
  (:Pressed
    (if (not (Variables|Default|GetIsUnableToMove))
      (Character|Jump)))
  (:Released
    (Character|StopJumping)))

(event Input|ActionEvents|InputActionManipulateTime
  (params (Key :type Key%20Structure :default "None"))
  (:Pressed
    (CallFunction|CheckNotificationWidget "Map_TimefoldRealm")
    (bind _returnvalue (Game|GetCurrentLevelName true))
    (if (Utilities|Enum|Equal(Enum) _returnvalue "Map_TimefoldRealm")
      (CallFunction|ApplyEffect 0 "/Game/Widgets/WB_TimeFreezeEffect.WB_TimeFreezeEffect_C"))))

(event Input|ActionEvents|InputActionEntangle
  (params (Key :type Key%20Structure :default "None"))
  (:Pressed
    (Variables|Default|SetIsEntangling true))
  (:Released
    (Variables|Default|SetIsEntangling false)))

(event Input|ActionEvents|InputActionPause
  (params (Key :type Key%20Structure :default "None"))
  (bind _returnvalue (Game|GetPlayerController 0))
  (bind _returnvalue_2 (Game|GetPlayerController 0))
  (:Pressed
    (bind _returnvalue_3 (Game|GetCurrentLevelName true))
    (if (Utilities|Enum|NotEqual(Enum) _returnvalue_3 "Map_Menu")
      (if (Variables|Default|GetIsPaused)
        (Variables|Default|SetIsPaused false)
        (Widget|RemovefromParent (Variables|Default|GetPauseWidget))
        (Game|SetGamePaused false)
        (Input|SetInputModeGameOnly _returnvalue_2 false)
        (Variables|/Script/Engine.PlayerController|SetbShowMouseCursor _returnvalue_2 false)
        (else
          (Variables|Default|SetIsPaused true)
          (bind _returnvalue_4 (UserInterface|CreateWidget "/Game/Widgets/WB_PauseMenu.WB_PauseMenu_C" _returnvalue))
          (bind _output_get (Variables|Default|SetPauseWidget _returnvalue_4))
          (UserInterface|Viewport|AddtoViewport _output_get 0)
          (Input|SetInputModeGameandUI _returnvalue (Variables|Default|GetPauseWidget) "DoNotLock" true false)
          (Variables|/Script/Engine.PlayerController|SetbShowMouseCursor (Game|GetPlayerController 0) true)
          (Game|SetGamePaused true))))))

(event Input|ActionEvents|InputActionInteractwithobject
  (params (Key :type Key%20Structure :default "None"))
  (:Pressed
    (Variables|Default|SetIsInteracting true))
  (:Released
    (Variables|Default|SetIsInteracting false)))

(event Input|ActionEvents|InputActionQuantumForge
  (params (Key :type Key%20Structure :default "None"))
  (:Pressed
    (CallFunction|CheckNotificationWidget "Map_QuantumForgeRealm")
    (bind _returnvalue (Game|GetCurrentLevelName true))
    (if (Utilities|Enum|Equal(Enum) _returnvalue "Map_QuantumForgeRealm")
      (CallFunction|ApplyEffect 1 "/Game/Widgets/WB_QuantumForgeEffect.WB_QuantumForgeEffect_C"))))

(event Input|ActionEvents|InputActionTryToChangeProperty
  (params (Key :type Key%20Structure :default "None"))
  (:Pressed
    (Variables|Default|SetIsChangingItemProperties true))
  (:Released
    (Variables|Default|SetIsChangingItemProperties false)))

(event Input|ActionEvents|InputActionTryToCombineItems
  (params (Key :type Key%20Structure :default "None"))
  (:Pressed
    (Variables|Default|SetIsCombiningItems true))
  (:Released
    (Variables|Default|SetIsCombiningItems false)))

(event Input|ActionEvents|InputActionCreateEcho
  (params (Key :type Key%20Structure :default "None"))
  (:Pressed
    (CallFunction|CheckNotificationWidget "Map_EchoRealm")
    (bind _returnvalue (Game|GetCurrentLevelName true))
    (if (Utilities|Enum|Equal(Enum) _returnvalue "Map_EchoRealm")
      (CallFunction|ApplyEffect 3 "/Game/Widgets/WB_EchoEffect.WB_EchoEffect_C"))))

(event Input|ActionEvents|InputActionInteractwithobjectshift
  (params (Key :type Key%20Structure :default "None"))
  (:Pressed
    (Variables|Default|SetIsInteractingShift true))
  (:Released
    (Variables|Default|SetIsInteractingShift false)))

(event Input|ActionEvents|InputActionQuantumEntanglement
  (params (Key :type Key%20Structure :default "None"))
  (:Pressed
    (CallFunction|CheckNotificationWidget "Map_EntanglementRealm")
    (bind _returnvalue (Game|GetCurrentLevelName true))
    (if (Utilities|Enum|Equal(Enum) _returnvalue "Map_EntanglementRealm")
      (CallFunction|ApplyEffect 2 "/Game/Widgets/WB_EntanglementEffect.WB_EntanglementEffect_C"))))

(event Input|ActionEvents|InputActionPossessClone
  (params (Key :type Key%20Structure :default "None"))
  (:Pressed
    (Variables|Default|SetIsChangingPossession true))
  (:Released
    (Variables|Default|SetIsChangingPossession false)))

(event Input|AxisEvents|InputAxisMoveRight
  (params (AxisValue :type Float%20%28single-precision%29))
  (if (not (Variables|Default|GetIsUnableToMove))
    (Pawn|Input|AddMovementInput "1.000000,0.000000,0.000000" AxisValue false)))

(fn ConstructionScript)

(fn HasAbility
  (params (Index :type Integer))
  (bind _asbp_game_instance (Utilities|Casting|CastToBP_GameInstance (Game|GetGameInstance)))
  (return (Utilities|Array|Get(acopy) (Variables|/Game/Blueprints/BP_GameInstance.BP_GameInstance_C|GetHasAbilities _asbp_game_instance) Index)))

(fn UpdateWidget
  (params (Index :type Integer) (AbilityWidget :type User%20Widget%20Class%20Reference) (CurrentWidget :type Object%20Object%20Reference))
  (if (Utilities|Array|Get(acopy) (Variables|Default|GetIsAbilityBeingUsed) Index)
    (Utilities|Array|SetArrayElem (Variables|Default|GetIsAbilityBeingUsed) Index false)
    (if (Utilities|IsValid CurrentWidget)
      (switch int Index
        (:0
          (bind _aswb_time_freeze_effect (Utilities|Casting|CastToWB_TimeFreezeEffect CurrentWidget))
          (Default|RemoveEffect _aswb_time_freeze_effect))
        (:1
          (bind _aswb_quantum_forge_effect (Utilities|Casting|CastToWB_QuantumForgeEffect CurrentWidget))
          (Default|RemoveEffect _aswb_quantum_forge_effect))
        (:2
          (bind _aswb_entanglement_effect (Utilities|Casting|CastToWB_EntanglementEffect CurrentWidget))
          (Default|RemoveEffect _aswb_entanglement_effect))
        (:3
          (bind _aswb_echo_effect (Utilities|Casting|CastToWB_EchoEffect CurrentWidget))
          (Default|RemoveEffect _aswb_echo_effect)))
      (Variables|Default|SetIsCooldownFinished true))
    (elif (Variables|Default|GetIsCooldownFinished)
      (Utilities|Array|SetArrayElem (Variables|Default|GetIsAbilityBeingUsed) Index true)
      (bind _returnvalue (UserInterface|CreateWidget AbilityWidget))
      (UserInterface|Viewport|AddtoViewport _returnvalue 0)
      (Variables|Default|SetIsCooldownFinished false)
      (return _returnvalue))))

(fn IsUsingAbilities
  (params (Index :type Integer))
  (for (_array_element _array_index) (Variables|Default|GetIsAbilityBeingUsed)
    (if (and _array_element (!= _array_index Index))
      (return false)))
  (return true))

(fn ApplyEffect
  (params (Index :type Integer) (Widget :type User%20Widget%20Class%20Reference))
  (bind _output (CallFunction|IsUsingAbilities Index))
  (bind _output_2 (CallFunction|HasAbility Index))
  (if (and _output_2 _output)
    (bind _newparam (CallFunction|UpdateWidget Index Widget (Variables|Default|GetCurrentWidget)))
    (Variables|Default|SetCurrentWidget _newparam)))

(fn Heal
  (params (Health :type Integer))
  (Variables|Default|SetHealth (Math|Integer|Min(Integer) (+ (Variables|Default|GetHealth) Health) 1000)))

(fn TakeDamage
  (params (Damage :type Integer) (IsDamageReduced :type Boolean))
  (if IsDamageReduced
    (Variables|Default|SetHealth (Math|Integer|Max(Integer) (- (Variables|Default|GetHealth) (- Damage 10))))
    (else
      (Variables|Default|SetHealth (Math|Integer|Max(Integer) (- (Variables|Default|GetHealth) Damage)))))
  (CallFunction|CheckforDeath))

(fn CheckNotificationWidget
  (params (MapName :type String))
  (Variables|Default|GetNotificationWidget
    (:then
      (bind _returnvalue (Game|GetCurrentLevelName true))
      (if (Utilities|Enum|Equal(Enum) _returnvalue MapName)
        (Widget|RemovefromParent (Variables|Default|GetNotificationWidget))))
    (:else)))