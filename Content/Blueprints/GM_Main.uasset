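; GM_Main is a game mode Blueprint that handles player death and respawn through flags stored in BP_GameInstance.
; Every tick it checks the death flag and, when it is set, opens Map_Main.
; On BeginPlay, a set death flag triggers a teleport to a fixed point and is cleared.
; The character's root is held Static for a short delay, then made Movable again and the reviving flag is cleared.
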(event Custom|Check%20Player%20Death
  (bind _asbp_game_instance (Utilities|Casting|CastToBP_GameInstance (Game|GetGameInstance)))
  (if (Variables|/Game/Blueprints/BP_GameInstance.BP_GameInstance_C|GetIsPlayerDead _asbp_game_instance)
    (Game|OpenLevel(byName) "Map_Main")))

(event EventBeginPlay
  (bind _returnvalue (Game|GetPlayerCharacter 0))
  (bind _rootcomponent (Variables|/Script/Engine.Actor|GetRootComponent _returnvalue))
  (bind _asbp_game_instance (Utilities|Casting|CastToBP_GameInstance (Game|GetGameInstance)))
  (if (Variables|/Game/Blueprints/BP_GameInstance.BP_GameInstance_C|GetIsPlayerDead _asbp_game_instance)
    (Transformation|Teleport (Game|GetPlayerCharacter 0) "210.000000,0.000000,10.000000" "0, 0, 0")
    (Transformation|SetMobility _rootcomponent "Static")
    (Variables|/Game/Blueprints/BP_GameInstance.BP_GameInstance_C|SetIsPlayerDead _asbp_game_instance false)
    (Utilities|FlowControl|Delay 2.0)
    (Transformation|SetMobility _rootcomponent "Movable")
    (bind _asbp_game_instance_2 (Utilities|Casting|CastToBP_GameInstance (Game|GetGameInstance)))
    (Variables|/Game/Blueprints/BP_GameInstance.BP_GameInstance_C|SetIsPlayerReviving _asbp_game_instance_2 false)))

(event EventTick
  (params (DeltaSeconds :type Float%20%28single-precision%29))
  (CallFunction|CheckPlayerDeath))

(fn ConstructionScript)