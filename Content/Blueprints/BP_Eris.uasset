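; BP_Eris is a dialogue NPC that shows a text prompt and talks to the player through a WB_Dialogue widget while overlapped.
; On a first meeting, flagged in BP_GameInstance, it opens dialogue automatically and locks player movement until the first line set ends.
; Tick polls the player's IsInteracting flag to advance lines, with later talks using a repeatable second set.
; Leaving the overlap resets both indices and closes the widget.
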(event Custom|TalkToPlayer
  (bind _asbp_sprite_character (Utilities|Casting|CastToBP_SpriteCharacter (Game|GetPlayerCharacter 0)))
  (if (Variables|/Game/Blueprints/BP_SpriteCharacter.BP_SpriteCharacter_C|GetIsInteracting _asbp_sprite_character)
    (CallFunction|Talk)
    (Variables|/Game/Blueprints/BP_SpriteCharacter.BP_SpriteCharacter_C|SetIsInteracting _asbp_sprite_character false)))

(event Collision|EventActorBeginOverlap
  (params (OtherActor :type Actor%20Object%20Reference))
  (Variables|Default|SetIsOverlapped true)
  (Development|SetHiddeninGame (Variables|Default|GetTextRender) false false)
  (bind _asbp_game_instance (Utilities|Casting|CastToBP_GameInstance (Game|GetGameInstance)))
  (Variables|Default|SetGI _asbp_game_instance)
  (if (Variables|/Game/Blueprints/BP_GameInstance.BP_GameInstance_C|GetIsFirstTime (Variables|Default|GetGI))
    (bind _asbp_sprite_character (Utilities|Casting|CastToBP_SpriteCharacter (Game|GetPlayerCharacter 0)))
    (Variables|/Game/Blueprints/BP_SpriteCharacter.BP_SpriteCharacter_C|SetIsUnableToMove _asbp_sprite_character true)
    (CallFunction|Talk)))

(event EventTick
  (params (DeltaSeconds :type Float%20%28single-precision%29))
  (if (Variables|Default|GetIsOverlapped)
    (CallFunction|TalktoPlayer)))

(event Collision|EventActorEndOverlap
  (params (OtherActor :type Actor%20Object%20Reference))
  (Variables|Default|SetIsOverlapped false)
  (bind _asbp_sprite_character (Utilities|Casting|CastToBP_SpriteCharacter (Game|GetPlayerCharacter 0)))
  (Variables|/Game/Blueprints/BP_SpriteCharacter.BP_SpriteCharacter_C|SetIsUnableToMove _asbp_sprite_character false)
  (Development|SetHiddeninGame (Variables|Default|GetTextRender) true false)
  (Variables|Default|SetFirstTalkIndex 0)
  (Variables|Default|SetSecondTalkIndex 0)
  (bind _ui (Variables|Default|GetUI)
    (:then
      (Widget|RemovefromParent _ui))
    (:else)))

(event EventTalk
  (bind _ui (Variables|Default|GetUI)
    (:then
      (Default|ClearDialogue _ui))
    (:else
      (bind _returnvalue (UserInterface|CreateWidget "/Game/Widgets/WB_Dialogue.WB_Dialogue_C" (Game|GetPlayerController 0)))
      (Variables|Default|SetUI _returnvalue)))
  (if (Variables|/Game/Blueprints/BP_GameInstance.BP_GameInstance_C|GetIsFirstTime (Variables|Default|GetGI))
    (if (UserInterface|Viewport|IsinViewport (Variables|Default|GetUI))
      _
      (else
        (UserInterface|Viewport|AddtoViewport (Variables|Default|GetUI) 0)))
    (Variables|/Game/Widgets/WB_Dialogue.WB_Dialogue_C|SetInputText (Variables|Default|GetUI) (Utilities|Array|Get(acopy) (Variables|Default|GetFirstDialogue) (Variables|Default|GetFirstTalkIndex)))
    (Default|PutText (Variables|Default|GetUI))
    (bind _result (Math|Integer|IncrementInt (Variables|Default|GetFirstTalkIndex))
      (:%20%20
        (if (>= _result (Utilities|Array|Length (Variables|Default|GetFirstDialogue)))
          (Variables|/Game/Blueprints/BP_GameInstance.BP_GameInstance_C|SetIsFirstTime (Variables|Default|GetGI) false)
          (bind _asbp_sprite_character (Utilities|Casting|CastToBP_SpriteCharacter (Game|GetPlayerCharacter 0)))
          (Variables|/Game/Blueprints/BP_SpriteCharacter.BP_SpriteCharacter_C|SetIsUnableToMove _asbp_sprite_character false)
          (Widget|RemovefromParent (Variables|Default|GetUI))
          (Development|SetHiddeninGame (Variables|Default|GetTextRender) false false))))
    (else
      (if (UserInterface|Viewport|IsinViewport (Variables|Default|GetUI))
        _
        (else
          (UserInterface|Viewport|AddtoViewport (Variables|Default|GetUI) 0)))
      (Variables|/Game/Widgets/WB_Dialogue.WB_Dialogue_C|SetInputText (Variables|Default|GetUI) (Utilities|Array|Get(acopy) (Variables|Default|GetSecondDialogue) (Variables|Default|GetSecondTalkIndex)))
      (Default|PutText (Variables|Default|GetUI))
      (bind _result_2 (Math|Integer|IncrementInt (Variables|Default|GetSecondTalkIndex))
        (:%20%20
          (if (>= _result_2 (Utilities|Array|Length (Variables|Default|GetSecondDialogue)))
            (Variables|Default|SetSecondTalkIndex 0)
            (Widget|RemovefromParent (Variables|Default|GetUI))))))))

(fn ConstructionScript)