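; BP_Machine is an interactable machine that the player toggles on and off, swapping its Paper2D flipbook to match.
; Actor overlap events, unfiltered by actor, set IsOverlapped and show or hide a text render.
; While overlapped, Tick calls Interact, which polls IsInteracting on the player's BP_SpriteCharacter, flips IsOn when it is set, then clears that flag to consume the input.
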(event Custom|Interact
  (bind _asbp_sprite_character (Utilities|Casting|CastToBP_SpriteCharacter (Game|GetPlayerCharacter 0)))
  (if (Variables|/Game/Blueprints/BP_SpriteCharacter.BP_SpriteCharacter_C|GetIsInteracting _asbp_sprite_character)
    (if (Variables|Default|GetIsOn)
      (Variables|Default|SetIsOn false)
      (Sprite|SetFlipbook (Variables|Default|GetSprite) "/Game/Assets/environment/props/Machine/FB_MachineOff.FB_MachineOff")
      (else
        (Variables|Default|SetIsOn true)
        (Sprite|SetFlipbook (Variables|Default|GetSprite) "/Game/Assets/environment/props/Machine/FB_MachineOn.FB_MachineOn")))
    (Variables|/Game/Blueprints/BP_SpriteCharacter.BP_SpriteCharacter_C|SetIsInteracting _asbp_sprite_character false)))

(event Collision|EventActorBeginOverlap
  (params (OtherActor :type Actor%20Object%20Reference))
  (Variables|Default|SetIsOverlapped true)
  (Development|SetHiddeninGame (Variables|Default|GetTextRender) false false))

(event EventTick
  (params (DeltaSeconds :type Float%20%28single-precision%29))
  (if (Variables|Default|GetIsOverlapped)
    (CallFunction|Interact)))

(event Collision|EventActorEndOverlap
  (params (OtherActor :type Actor%20Object%20Reference))
  (Variables|Default|SetIsOverlapped false)
  (Development|SetHiddeninGame (Variables|Default|GetTextRender) true false))

(fn ConstructionScript)