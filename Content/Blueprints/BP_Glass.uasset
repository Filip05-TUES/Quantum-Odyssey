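; BP_Glass is a flipbook-sprite glass character that the player can pick up, drop or duplicate.
; Overlap with BP_SpriteCharacter shows a prompt and enables interaction, polled on Tick through the player's IsInteracting flag.
; While carried, it follows the player's location every frame and registers as the held item.
; With the player's ability at index 1 active, interacting instead spawns a copy with the same flipbook, launched upward and randomly sideways.
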(event Custom|Interact
  (if (Utilities|Array|Get(acopy) (Variables|/Game/Blueprints/BP_SpriteCharacter.BP_SpriteCharacter_C|GetIsAbilityBeingUsed (Variables|Default|GetPlayer)) 1)
    (CallFunction|TryDuplicate)
    (else
      (CallFunction|PickUp))))

(event Custom|UpdateLocation
  (if (Variables|Default|GetIsPicked)
    (Transformation|SetActorLocation (+ (Transformation|GetActorLocation (Game|GetPlayerCharacter 0)) "0.000000,0.000000,10.000000") false false)))

(event Custom|SetText
  (if (Utilities|Array|Get(acopy) (Variables|/Game/Blueprints/BP_SpriteCharacter.BP_SpriteCharacter_C|GetIsAbilityBeingUsed (Variables|Default|GetPlayer)) 1)
    (Variables|Default|SetCurrentText "[I] Duplicate")
    (elif (Variables|Default|GetIsPicked)
      (Variables|Default|SetCurrentText "[I] Drop")
      (else
        (Variables|Default|SetCurrentText "[I] Pick Up")))))

(event Custom|PickUp
  (if (Variables|/Game/Blueprints/BP_SpriteCharacter.BP_SpriteCharacter_C|GetIsInteracting (Variables|Default|GetPlayer))
    (if (Variables|Default|GetIsPicked)
      (Variables|Default|SetIsPicked false)
      (Variables|/Game/Blueprints/BP_SpriteCharacter.BP_SpriteCharacter_C|SetIsHoldingSomething (Variables|Default|GetPlayer) false)
      (Variables|/Game/Blueprints/BP_SpriteCharacter.BP_SpriteCharacter_C|SetItemHeld (Variables|Default|GetPlayer) 0)
      (Variables|/Game/Blueprints/BP_SpriteCharacter.BP_SpriteCharacter_C|SetIsInteracting (Variables|Default|GetPlayer) false :!label _label)
      (elif (not (Variables|/Game/Blueprints/BP_SpriteCharacter.BP_SpriteCharacter_C|GetIsHoldingSomething (Variables|Default|GetPlayer)))
        (Variables|Default|SetIsPicked true)
        (Variables|/Game/Blueprints/BP_SpriteCharacter.BP_SpriteCharacter_C|SetIsHoldingSomething (Variables|Default|GetPlayer) true)
        (Variables|/Game/Blueprints/BP_SpriteCharacter.BP_SpriteCharacter_C|SetItemHeld (Variables|Default|GetPlayer) self)
        (goto _label)))))

(event EventBeginPlay
  (Variables|Default|SetPlayer (.AsBP%20Sprite%20Character (Utilities|Casting|CastToBP_SpriteCharacter (Game|GetPlayerCharacter 0)))))

(event Collision|EventActorBeginOverlap
  (params (OtherActor :type Actor%20Object%20Reference))
  (if (== (Utilities|GetClass OtherActor) "/Game/Blueprints/BP_SpriteCharacter.BP_SpriteCharacter_C")
    (Variables|Default|SetIsOverlapped true)
    (Development|SetHiddeninGame (Variables|Default|GetTextRender) false false)))

(event EventTick
  (params (DeltaSeconds :type Float%20%28single-precision%29))
  (CallFunction|SetText)
  (Rendering|Components|TextRender|SetText (Variables|Default|GetTextRender) (Variables|Default|GetCurrentText))
  (CallFunction|UpdateLocation)
  (if (Variables|Default|GetIsOverlapped)
    (CallFunction|Interact)))

(event Collision|EventActorEndOverlap
  (params (OtherActor :type Actor%20Object%20Reference))
  (if (== (Utilities|GetClass OtherActor) "/Game/Blueprints/BP_SpriteCharacter.BP_SpriteCharacter_C")
    (Variables|Default|SetIsOverlapped false)
    (Development|SetHiddeninGame (Variables|Default|GetTextRender) true false)))

(fn ConstructionScript)

(fn TryDuplicate
  (if (Variables|/Game/Blueprints/BP_SpriteCharacter.BP_SpriteCharacter_C|GetIsInteracting (Variables|Default|GetPlayer))
    (bind _returnvalue (Game|SpawnActorfromClass "BP_Glass_C" (Transformation|GetActorTransform) "Undefined" "MultiplyWithRoot" 0 0))
    (Pawn|SpawnDefaultController _returnvalue)
    (Sprite|SetFlipbook (Variables|/Script/Paper2D.PaperCharacter|GetSprite _returnvalue) (Class|PaperFlipbookComponent|GetFlipbook (Variables|Default|GetSprite)))
    (Character|LaunchCharacter _returnvalue (Math|Vector|MakeVector (* (Math|Float|SelectFloat 1.0 -1.0 (Math|Random|RandomBool)) (Math|Random|RandomFloatinRange 2e+02 1e+02)) 0.0 2e+02) false false)
    (Variables|/Game/Blueprints/BP_SpriteCharacter.BP_SpriteCharacter_C|SetIsInteracting (Variables|Default|GetPlayer) false)
    (return true)
    (else
      (return false))))