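; Quantum Devourer boss that fights the player by picking a random move whenever MakeRandomMove is called: block, fire, heal or laser.
; Block refunds the last damage taken, laser also sets a burn duration, and each move swaps flipbooks before returning to idle.
; While entangled, the boss's attacks also damage itself and its heal also heals the player.
; A death check precedes every move except block, playing the death animation and setting the player's capsule to Movable.
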(event Custom|CheckForDeath
  (bind _sprite (Variables|Default|GetSprite))
  (if (<= (Variables|Default|GetHealth) 0)
    (Variables|Default|SetIsDead true)
    (Sprite|SetFlipbook _sprite "/Game/Assets/sprites/QuantumDevourer/death/FB_DevourerDeath.FB_DevourerDeath")
    (Components|Timeline|SetLooping _sprite false)
    (Transformation|SetActorLocation "700.000000,0.000000,-502.000000" false false)
    (Utilities|FlowControl|Delay 2.0)
    (Transformation|SetMobility (Variables|/Script/Engine.Character|GetCapsuleComponent (Game|GetPlayerCharacter 0)) "Movable")))

(event Custom|MakeRandomMove
  (switch int (Math|Random|RandomInteger 4)
    (:0
      (CallFunction|BlockDamage))
    (:1
      (CallFunction|CheckforDeath)
      (if (not (Variables|Default|GetIsDead))
        (CallFunction|Fire)))
    (:2
      (CallFunction|CheckforDeath)
      (if (not (Variables|Default|GetIsDead))
        (CallFunction|Heal)))
    (:3
      (CallFunction|CheckforDeath)
      (if (not (Variables|Default|GetIsDead))
        (CallFunction|Laser)))))

(event Custom|Heal
  (Variables|Default|SetHealth (Math|Integer|Min(Integer) (+ (Variables|Default|GetHealth) 100) 1000))
  (Variables|Default|SetDamageTaken 0)
  (Sprite|SetFlipbook (Variables|Default|GetSprite) "/Game/Assets/sprites/QuantumDevourer/healing/FB_Healing.FB_Healing")
  (if (> (Variables|Default|GetEntangleDuration) 0)
    (Default|Heal (.AsBP%20Sprite%20Character (Utilities|Casting|CastToBP_SpriteCharacter (Game|GetPlayerCharacter 0))) 100))
  (Utilities|FlowControl|Delay 2.0)
  (Sprite|SetFlipbook (Variables|Default|GetSprite) "/Game/Assets/sprites/QuantumDevourer/idle/FB_BossIdle.FB_BossIdle"))

(event Custom|BlockDamage
  (bind _sprite (Variables|Default|GetSprite))
  (bind _sprite_2 (Variables|Default|GetSprite))
  (Variables|Default|SetHealth (Math|Integer|Min(Integer) (+ (Variables|Default|GetHealth) (Variables|Default|GetDamageTaken)) 1000))
  (Variables|Default|SetDamageTaken 0)
  (Sprite|SetFlipbook _sprite "/Game/Assets/sprites/QuantumDevourer/block/FB_Block.FB_Block")
  (Components|Timeline|SetLooping _sprite false)
  (Utilities|FlowControl|Delay 2.0)
  (Sprite|SetFlipbook _sprite_2 "/Game/Assets/sprites/QuantumDevourer/idle/FB_BossIdle.FB_BossIdle")
  (Components|Timeline|SetLooping _sprite_2 true)
  (Audio|Components|Audio|Play _sprite_2))

(event Custom|Fire
  (bind _sprite (Variables|Default|GetSprite))
  (bind _sprite_2 (Variables|Default|GetSprite))
  (Default|TakeDamage (.AsBP%20Sprite%20Character (Utilities|Casting|CastToBP_SpriteCharacter (Game|GetPlayerCharacter 0))) 130)
  (Variables|Default|SetDamageTaken 0)
  (Sprite|SetFlipbook _sprite_2 "/Game/Assets/sprites/QuantumDevourer/fire/FB_Fire.FB_Fire")
  (Components|Timeline|SetLooping _sprite_2 false)
  (Variables|Default|SetIsUsingArm true)
  (if (> (Variables|Default|GetEntangleDuration) 0)
    (CallFunction|TakeDamage 130))
  (Utilities|FlowControl|Delay 2.0)
  (Sprite|SetFlipbook _sprite "/Game/Assets/sprites/QuantumDevourer/idle/FB_BossIdle.FB_BossIdle")
  (Components|Timeline|SetLooping _sprite true)
  (Audio|Components|Audio|Play _sprite)
  (Variables|Default|SetIsUsingArm false))

(event Custom|Laser
  (bind _sprite (Variables|Default|GetSprite))
  (bind _sprite_2 (Variables|Default|GetSprite))
  (Variables|Default|SetBurnDuration 3)
  (Default|TakeDamage (.AsBP%20Sprite%20Character (Utilities|Casting|CastToBP_SpriteCharacter (Game|GetPlayerCharacter 0))) 50)
  (Variables|Default|SetDamageTaken 0)
  (Sprite|SetFlipbook _sprite "/Game/Assets/sprites/QuantumDevourer/laser/FB_Laser.FB_Laser")
  (Components|Timeline|SetLooping _sprite false)
  (Variables|Default|SetIsUsingLaser true)
  (if (> (Variables|Default|GetEntangleDuration) 0)
    (CallFunction|TakeDamage 50))
  (Utilities|FlowControl|Delay 2.0)
  (Sprite|SetFlipbook _sprite_2 "/Game/Assets/sprites/QuantumDevourer/idle/FB_BossIdle.FB_BossIdle")
  (Components|Timeline|SetLooping _sprite_2 true)
  (Audio|Components|Audio|Play _sprite_2)
  (Variables|Default|SetIsUsingLaser false))

(fn ConstructionScript)

(fn TakeDamage
  (params (Damage :type Integer))
  (Variables|Default|SetDamageTaken Damage)
  (Variables|Default|SetHealth (Math|Integer|Max(Integer) (- (Variables|Default|GetHealth) Damage))))